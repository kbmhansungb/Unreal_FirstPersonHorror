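; RotateCamera is a trigger volume actor that redirects the horror player's camera when BP_HorrorPlayerCharacter begins overlapping its Box.
; The UseFocus flag chooses between the player's focus functions and RotateCameraToLookAt, with CallFocusIn further selecting FocusIn or FocusOut.
; FocusIn and the look-at rotation target the location of the FocusActor child actor, and all three calls share the Duration variable.
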(event OnComponentBeginOverlap(Box)
  (params (OverlappedComponent :type Primitive%20Component%20Object%20Reference) (OtherActor :type Actor%20Object%20Reference) (OtherComp :type Primitive%20Component%20Object%20Reference) (OtherBodyIndex :type Integer) (bFromSweep :type Boolean) (SweepResult :type Hit%20Result%20Structure%20%28by%20ref%29))
  (bind _focusactor (Variables|Default|GetFocusActor))
  (bind _duration (Variables|Default|GetDuration))
  (bind _childactor (Variables|/Script/Engine.ChildActorComponent|GetChildActor _focusactor))
  (bind _returnvalue (Transformation|GetActorLocation _childactor))
  (bind _asbp_horror_player_character (Utilities|Casting|CastToBP_HorrorPlayerCharacter OtherActor))
  (if (Variables|Default|GetUseFocus)
    (if (Variables|Default|GetCallFocusIn)
      (Class|HorrorPlayerCharacter|Focusin _asbp_horror_player_character _returnvalue _duration)
      (else
        (Class|HorrorPlayerCharacter|FocusOut _asbp_horror_player_character _duration)))
    (else
      (Class|HorrorPlayerCharacter|RotateCameratoLookat _asbp_horror_player_character _returnvalue _duration))))

(event EventBeginPlay)

(event Collision|EventActorBeginOverlap
  (params (OtherActor :type Actor%20Object%20Reference)))

(event EventTick
  (params (DeltaSeconds :type Float%20%28single-precision%29)))

(fn ConstructionScript)